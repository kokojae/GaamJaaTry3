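; BP_TestGaamjaa provides click-to-move and touch-to-move control that sends player 0 to the point under the cursor or finger.
; SetDestination and first-finger touch each open a gate on press and close it on release.
; While a gate is open, Tick runs a complex Visibility trace every frame and passes the hit to MoveToHitLocation, which calls SimpleMoveToLocation on the player controller.
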(event EventBeginPlay)

(event Collision|EventActorBeginOverlap
  (params (OtherActor :type Actor%20Object%20Reference)))

(event EventTick
  (params (DeltaSeconds :type Float%20%28single-precision%29))
  (bind _returnvalue (Game|GetPlayerController 0))
  (Utilities|FlowControl|Sequence
    (:then_0
      (Utilities|FlowControl|Gate true
        (:Exit
          (CallFunction|MovetoHitLocation (.HitResult (Game|Player|GetHitResultUnderCursorbyChannel _returnvalue "TraceTypeQuery1" true))))))
    (:then_1
      (Utilities|FlowControl|Gate true
        (:Exit
          (CallFunction|MovetoHitLocation (.HitResult (Class|PlayerController|GetHitResultUnderFingerbyChannel _returnvalue (stale Input|TouchEvents|InputTouch FingerIndex) "TraceTypeQuery1" true))))))))

(event Input|ActionEvents|InputActionSetDestination
  (params (Key :type Key%20Structure))
  (:Pressed
    (Utilities|FlowControl|Gate true) ; enters at Open
  )
  (:Released
    (Utilities|FlowControl|Gate true) ; enters at Close
  ))

(event Input|TouchEvents|InputTouch
  (params (Location :type Vector) (FingerIndex :type ETouchIndex%20Enum))
  (bind _returnvalue (Utilities|Enum|Equal(Enum) FingerIndex "Touch1"))
  (:Pressed
    (if _returnvalue
      (Utilities|FlowControl|Gate true) ; enters at Open
    ))
  (:Released
    (if _returnvalue
      (Utilities|FlowControl|Gate true) ; enters at Close
    )))

(fn ConstructionScript)

(fn MovetoHitLocation
  (params (Hit :type Hit%20Result%20Structure))
  (AI|Navigation|SimpleMovetoLocation (Game|GetPlayerController 0) (.Location (Collision|BreakHitResult Hit))))